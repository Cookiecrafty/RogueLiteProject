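; Master room Blueprint for the procedural dungeon, implementing a trap room that runs enemy waves until its closed doors reopen.
; WaveBegin stores the given doors, spawns random-class enemies inside OverlapTrapBox and binds their dispatchers to count down EnemyLeft.
; When a wave is cleared, it starts the next with a multiplied enemy count, or opens the doors if none remain.
; BeginPlay's RoomType switch is empty, and Tick prints EnemyLeft for debugging.
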(event Custom|WaveBegin
  (params (DoorClosed :type Array%20of%20BP%20Door%20Object%20References))
  (bind _overlaptrapbox (Variables|Default|GetOverlapTrapBox))
  ;[1 0.1765 0.1666] Trap Room
  (Variables|Default|SetClosedDoor DoorClosed)
  (for _index (range 0 (Variables|Default|GetNumberofEnemyPerWave))
    (bind _returnvalue (Game|SpawnActorfromClass (.OutItem (Utilities|Array|Random (Variables|Default|GetClass))) (Math|Transform|MakeTransform (Math|Random|RandomPointinBoundingBox (Transformation|GetWorldLocation _overlaptrapbox) (Components|Box|GetScaledBoxExtent _overlaptrapbox)) "0, 0, 0" "1.000000,1.000000,1.000000") "AdjustIfPossibleButAlwaysSpawn" "MultiplyWithRoot" 0 "0.000000,0.000000,0.000000" self 0))
    (EventDispatchers|BindEventtoUpdateSpawnerDispatcher _returnvalue (EventDispatchers|CreateEvent :!event Custom|UpdateSpawner))
    (Utilities|Array|Add (Variables|Default|GetEnemyREF) 0)
    (Variables|Default|SetEnemyLeft (+ (Variables|Default|GetNumberofEnemyPerWave) 1))))

(event Custom|UpdateSpawner
  ;[1 0.1765 0.1666] Trap Room
  (Math|Integer|DecrementInt (Variables|Default|GetEnemyLeft)
    (:%20%20
      (if (== (Variables|Default|GetEnemyLeft) 0)
        (Development|PrintString "TOUT EST MORT")
        (if (== (Variables|Default|GetWaveNumber) 0)
          (for _array_element (Variables|Default|GetClosedDoor)
            (Default|OpenDoor _array_element))
          (Development|PrintString "Open Doors")
          (else
            (Math|Integer|DecrementInt (Variables|Default|GetWaveNumber)
              (:%20%20
                (Variables|Default|SetNumberofEnemyPerWave (Math|Float|Round (* (Variables|Default|GetNumberofEnemyPerWave) (Variables|Default|GetMultiplierEachWave))))
                (CallFunction|WaveBegin (Variables|Default|GetClosedDoor))))))
        (else
          (Development|PrintString "- 1 ennemi"))))))

(event EventTick
  (params (DeltaSeconds :type Float%20%28single-precision%29))
  (Development|PrintString (Utilities|String|ToString(Integer) (Variables|Default|GetEnemyLeft)) true true "(R=1.000000,G=0.000000,B=0.815304,A=1.000000)" 0.0))

(event EventBeginPlay
  (switch Utilities|FlowControl|Switch|SwitchonETypeRoom (Variables|Default|GetRoomType)))

(fn ConstructionScript)