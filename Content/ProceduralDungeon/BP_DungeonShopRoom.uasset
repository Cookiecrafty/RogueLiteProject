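; Procedural dungeon room that hosts an in-game shop.
; On BeginPlay it runs the parent logic, spawns BP_ShopInGame at its Arrow component's world transform regardless of collisions, and keeps a reference to it.
; When the room is destroyed, it destroys that shop actor too, so the shop's lifetime follows the room's.
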(event EventBeginPlay
  (|CallParentFunction)
  (bind _returnvalue (Game|SpawnActorfromClass "/Game/ThirdPerson/Shop/BP_ShopInGame.BP_ShopInGame_C" (Transformation|GetWorldTransform (Variables|Default|GetArrow)) "AlwaysSpawn" "MultiplyWithRoot" 0 0))
  (Variables|Default|SetShopREF _returnvalue))

(event Collision|EventActorBeginOverlap
  (params (OtherActor :type Actor%20Object%20Reference))
  (|CallParentFunction OtherActor) ; This node is disabled and will not be called.\nDrag off pins to build functionality.
)

(event EventTick
  (params (DeltaSeconds :type Float%20%28single-precision%29))
  (|CallParentFunction DeltaSeconds) ; This node is disabled and will not be called.\nDrag off pins to build functionality.
)

(event EventDestroyed
  (Actor|DestroyActor (Variables|Default|GetShopREF)))

(fn ConstructionScript
  (|CallParentFunction))