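; BP_DungeonPortalRoom is a procedural dungeon room that contains a portal.
; On BeginPlay it runs the parent logic, then always spawns a BP_Portal at its Arrow component's transform, with the yaw turned 180 degrees.
; The Arrow serves as the placement marker; overlap and tick events are unused, and construction defers to the parent.
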(event EventBeginPlay
  (bind _arrow (Variables|Default|GetArrow))
  (bind _returnvalue (Transformation|GetWorldTransform _arrow))
  (|CallParentFunction)
  (Game|SpawnActorfromClass "/Game/ThirdPerson/BP_Portal.BP_Portal_C" (Math|Transform|MakeTransform (.location _returnvalue) (Math|Rotator|MakeRotator (.roll (.rotation _returnvalue)) (.pitch (.rotation _returnvalue)) (+ (.yaw (.rotation _returnvalue)) 1.8e+02)) (.scale _returnvalue)) "AlwaysSpawn" "MultiplyWithRoot" 0 17 0))

(event Collision|EventActorBeginOverlap
  (params (OtherActor :type Actor%20Object%20Reference))
  (|CallParentFunction OtherActor) ; This node is disabled and will not be called.\nDrag off pins to build functionality.
)

(event EventTick
  (params (DeltaSeconds :type Float%20%28single-precision%29))
  (|CallParentFunction DeltaSeconds) ; This node is disabled and will not be called.\nDrag off pins to build functionality.
)

(fn ConstructionScript
  (|CallParentFunction))