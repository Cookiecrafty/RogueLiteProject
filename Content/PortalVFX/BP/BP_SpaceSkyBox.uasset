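; BP_SpaceSkyBox is a space skybox actor in the PortalVFX content whose brightness is animated when play begins.
; The construction script applies MI_Space to the static mesh.
; BeginPlay swaps in a dynamic instance of that material, then plays the Brightness timeline, which drives the material's Brightness scalar parameter on each update.
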(event EventBeginPlay
  (bind _returnvalue (Rendering|Material|CreateDynamicMaterialInstance "/Game/PortalVFX/Material/Level/MI_Space.MI_Space" "None" :!class /Script/Engine.KismetMaterialLibrary))
  (Variables|Default|SetSpace _returnvalue)
  (Rendering|Material|SetMaterial (Variables|Default|GetStaticMesh) 0 (Variables|Default|GetSpace))
  (bind _newtrack_0 (Timeline|Brightness Play)
    (:Update
      (Rendering|Material|SetScalarParameterValue (Variables|Default|GetSpace) "Brightness" _newtrack_0 :!class /Script/Engine.MaterialInstanceDynamic))))

(fn ConstructionScript
  (Rendering|Material|SetMaterial (Variables|Default|GetStaticMesh) 0 "/Game/PortalVFX/Material/Level/MI_Space.MI_Space"))