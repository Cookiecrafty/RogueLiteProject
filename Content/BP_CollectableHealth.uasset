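; BP_CollectableHealth is a health pickup that heals the third-person player character when touched.
; When its Box is overlapped by BP_ThirdPersonCharacter, a DoOnce adds a fixed amount to Health, clamped to HealthMax.
; It then updates the character's HUD, plays a 2D pickup sound and destroys itself.
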(event OnComponentBeginOverlap(Box)
  (params (OverlappedComponent :type Primitive%20Component%20Object%20Reference) (OtherActor :type Actor%20Object%20Reference) (OtherComp :type Primitive%20Component%20Object%20Reference) (OtherBodyIndex :type Integer) (bFromSweep :type Boolean) (SweepResult :type Hit%20Result%20Structure%20%28by%20ref%29))
  (bind _asbp_third_person_character (Utilities|Casting|CastToBP_ThirdPersonCharacter OtherActor))
  (Utilities|FlowControl|DoOnce false
    (:Completed
      (bind _output_get (Variables|/Game/ThirdPerson/Blueprints/BP_ThirdPersonCharacter.BP_ThirdPersonCharacter_C|SetHealth _asbp_third_person_character (Math|Float|Clamp(Float) (+ (Variables|/Game/ThirdPerson/Blueprints/BP_ThirdPersonCharacter.BP_ThirdPersonCharacter_C|GetHealth _asbp_third_person_character) 5.0) 0.0 (Variables|/Game/ThirdPerson/Blueprints/BP_ThirdPersonCharacter.BP_ThirdPersonCharacter_C|GetHealthMax _asbp_third_person_character))))
      (Default|UpdateHP (Variables|/Game/ThirdPerson/Blueprints/BP_ThirdPersonCharacter.BP_ThirdPersonCharacter_C|GetHUD_REF _asbp_third_person_character) _output_get)
      (Audio|PlaySound2D "/Game/SoundsFX/FX_Health.FX_Health" 1.0 1.0 0.0 0 0)
      (Actor|DestroyActor))))

(fn ConstructionScript)